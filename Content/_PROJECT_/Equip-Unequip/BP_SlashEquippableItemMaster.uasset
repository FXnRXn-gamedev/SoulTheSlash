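; Base Blueprint for equippable items, handling held-pivot alignment and physics state for equip and unequip.
; SetPivot offsets the actor by the HeldPivot location while held, flipping it 180 degrees when FlipOnEquipped is set, and zeroes the relative transform otherwise.
; TogglePhysics switches simulation on the Main component.
; The construction script applies the Swing and Twist variables as angular limits on its PhysicsConstraint.
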(event `self.SetPivot`
  (params (bHeld :type Boolean))
  (bind _returnvalue (and bHeld (`self.FlipOnEquipped`)))
  ;[0.0518 0.4678 0.1435] Set rotation and location to the hel;d pivot so that if it has different pivot when equipped rotate actor 180 and flipped
  (`self.K2_SetActorRelativeRotation` (`KismetMathLibrary.SelectRotator` (struct :`Pitch` 180.0) (struct) _returnvalue))
  (`self.K2_SetActorRelativeLocation` (`KismetMathLibrary.SelectVector` (* (`SceneComponent.RelativeLocation` (`self.Held Pivot`)) (`KismetMathLibrary.SelectFloat` 1.0 -1.0 _returnvalue)) (0.0 0.0 0.0) bHeld)))

(event `self.TogglePhysics`
  (params (bEnable :type Boolean))
  ;[0.0518 0.4678 0.1435] Physics
  (`PrimitiveComponent.SetSimulatePhysics` (`self.Main`) bEnable))

(fn `UserConstructionScript`
  (bind _physicsconstraint (`self.PhysicsConstraint`))
  ;[0 0.15 0.1232 0.5] Set default swing/twist
  (`PhysicsConstraintComponent.SetAngularSwing1Limit` _physicsconstraint "ACM_Limited" (`self.Swing`))
  (`PhysicsConstraintComponent.SetAngularTwistLimit` _physicsconstraint "ACM_Limited" (`self.Twist`)))