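; Master Blueprint for an equippable item, apparently a base for child items, with all of its events and its construction script currently empty.
; Disconnected nodes sketch a held-pivot offset with optional 180-degree flip on equip, inner and outer interaction sphere sizing, and angular swing/twist constraint limits.
; None of that logic runs, and the SetPivot and TogglePhysics events are stubs in this graph.
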(event `self.ReceiveBeginPlay`)

(event `self.SetPivot`
  (params (bHeld :type Boolean))
  ;[0.0518 0.4678 0.1435] Set rotation and location to the hel;d pivot so that if it has different pivot when equipped rotate actor 180 and flipped
)

(event `self.TogglePhysics`
  (params (bEnable :type Boolean))
  ;[0.0518 0.4678 0.1435] Physics
)

(fn `UserConstructionScript`)